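; BP_Deadeye is an enemy Blueprint that sets up its Gameplay Ability System loadout when play begins.
; After a brief delay, only the authority grants the ranged Deadlock ability and tries to activate abilities tagged Stat.AI.
; It then applies the Deadlock init and full-health effects to itself, after that activation attempt.
; The GiveMeAbilities function is an empty stub; GiveAbilities does the work.
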(event `GiveAbilities`
  (bind _returnvalue (`self.GetAbilitySystemComponent`))
  (`self.SetupAbilitySystemComponent`)
  (`AbilitySystemComponent.K2_GiveAbility` _returnvalue "/Game/Blueprint/GameplayEffects/Enemies/Deadlock/GA_Deadlock_ranged_BP.GA_Deadlock_ranged_BP_C" 1 -1)
  (`AbilitySystemComponent.TryActivateAbilitiesByTag` _returnvalue (`self.AbilityTagContainer`) true)
  (`AbilitySystemComponent.BP_ApplyGameplayEffectToSelf` :`self` _returnvalue :`GameplayEffectClass` "/Game/Blueprint/GameplayEffects/Enemies/Deadlock/GE_DeadlockInit.GE_DeadlockInit_C" :`Level` 1.0)
  (`AbilitySystemComponent.BP_ApplyGameplayEffectToSelf` :`self` _returnvalue :`GameplayEffectClass` "/Game/Blueprint/GameplayEffects/GE_FullHealth.GE_FullHealth_C" :`Level` 1.0))

(event `self.ReceiveBeginPlay`
  (set `self.AbilityTagContainer` (struct :`GameplayTags` (struct :`(TagName` "stat.AI"))))
  (`KismetSystemLibrary.Delay` 0.1)
  (if (`self.HasAuthority`)
    (`self.GiveAbilities`)))

(fn `GiveMeAbilities`)

(fn `UserConstructionScript`)