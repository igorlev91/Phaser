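; BP_FadeMesh is an actor component that fades the owner's static mesh in and out of a fade material look.
; StartFade swaps in dynamic instances of FadeMaterials, created once and reused, while EndFade reverses the fade.
; Tick moves the fade at constant speed, writes an eased "Fade" parameter up to MaxFade, and disables itself at either end.
; Original materials, cached on BeginPlay, return once fully faded back.
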(event `self.ReceiveBeginPlay`
  (`self.InitFade`))

(event `self.ReceiveTick`
  (params (DeltaSeconds :type "Float (single-precision)"))
  (`self.TickFade` DeltaSeconds))

(fn `EndFade`
  (`/Engine/EditorBlueprintResources/StandardMacros.IsValid` (`self.MyMesh`)
    (:`Is Valid`
      (if (> (`KismetArrayLibrary.Array_Length` (`self.DefaultMaterials`)) 0)
        (if (> (`KismetArrayLibrary.Array_Length` (`self.FadeDynamicMaterials`)) 0)
          (set `self.bFading` false)
          (`self.SetComponentTickEnabled` true))))))

(fn `InitFade`
  (locals (NewLocalVar :type "StaticMeshComponent Object Reference"))
  (set `self.MyMesh` (`Actor.GetComponentByClass` (`self.GetOwner`) "/Script/Engine.StaticMeshComponent"))
  (bind _mymesh (`self.MyMesh`)
    (:`then`
      (set `self.DefaultMaterials` (`MeshComponent.GetMaterials` _mymesh)))
    (:`else`)))

(fn `SetDefaultMaterial`
  (`/Engine/EditorBlueprintResources/StandardMacros.IsValid` (`self.MyMesh`)
    (:`Is Valid`
      (if (> (`KismetArrayLibrary.Array_Length` (`self.DefaultMaterials`)) 0)
        (for (_array_element _array_index) (`self.DefaultMaterials`)
          (`PrimitiveComponent.SetMaterial` (`self.MyMesh`) _array_index _array_element))))))

(fn `StartFade`
  (`/Engine/EditorBlueprintResources/StandardMacros.IsValid` (`self.MyMesh`)
    (:`Is Valid`
      (if (> (`KismetArrayLibrary.Array_Length` (`self.FadeMaterials`)) 0)
        (if (not (> (`KismetArrayLibrary.Array_Length` (`self.FadeDynamicMaterials`)) 0))
          (for _array_element (`self.FadeMaterials`)
            (bind _returnvalue (`KismetMaterialLibrary.CreateDynamicMaterialInstance` _array_element))
            (`KismetArrayLibrary.Array_Add` (`self.FadeDynamicMaterials`) _returnvalue)))
        (for (_array_element_2 _array_index) (`self.FadeDynamicMaterials`)
          (`PrimitiveComponent.SetMaterial` (`self.MyMesh`) _array_index _array_element_2))
        (set `self.bFading` true)
        (`self.SetComponentTickEnabled` true)))))

(fn `TickFade`
  (params (DeltaTime :type "Float (double-precision)"))
  (set `self.currentFade` (`KismetMathLibrary.FInterpTo_Constant` (`self.currentFade`) (`KismetMathLibrary.SelectFloat` 1.0 0.0 (`self.bFading`)) (`local.DeltaTime`) (`self.interpSpeedFade`)))
  (for _array_element (`self.FadeDynamicMaterials`)
    (`MaterialInstanceDynamic.SetScalarParameterValue` _array_element "Fade" (`KismetMathLibrary.FInterpEaseInOut` 0.0 (`self.maxFade`) (`self.currentFade`) 2.0)))
  (if (`self.bFading`)
    (if (>= (`self.currentFade`) 1.0)
      (`self.SetComponentTickEnabled` false))
    (elif (<= (`self.currentFade`) 0.0)
      (`self.SetComponentTickEnabled` false)
      (`self.SetDefaultMaterial`))))