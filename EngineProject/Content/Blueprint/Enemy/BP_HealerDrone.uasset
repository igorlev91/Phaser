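; BP_HealerDrone is an enemy drone that sets up its Gameplay Ability System loadout for healing and flying.
; Shortly after BeginPlay, it initializes the ability system component and grants the enemy heal and flying abilities.
; It then attempts to activate abilities matching the Stat.AI tag container and applies init and full-health gameplay effects to itself.
; The setup event keeps a SpiderDrone name, and GiveMeAbilities is an empty stub.
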(event `SpiderDroneAbilities`
  (bind _returnvalue (`self.GetAbilitySystemComponent`))
  (`self.SetupAbilitySystemComponent`)
  (`AbilitySystemComponent.K2_GiveAbility` _returnvalue "/Game/Blueprint/GameplayEffects/Enemies/HealingDrone/GA_EnemyHeal_BP.GA_EnemyHeal_BP_C" 1 -1)
  (`AbilitySystemComponent.K2_GiveAbility` _returnvalue "/Game/Blueprint/GameplayEffects/Enemies/HealingDrone/GA_Flying_BP.GA_Flying_BP_C" 1 -1)
  (`AbilitySystemComponent.TryActivateAbilitiesByTag` _returnvalue (`self.AbilityTagContainer`) true)
  (`AbilitySystemComponent.BP_ApplyGameplayEffectToSelf` :`self` _returnvalue :`GameplayEffectClass` "/Game/Blueprint/GameplayEffects/Enemies/HealingDrone/GE_HealingdroneInit.GE_HealingdroneInit_C" :`Level` 1.0)
  (`AbilitySystemComponent.BP_ApplyGameplayEffectToSelf` :`self` _returnvalue :`GameplayEffectClass` "/Game/Blueprint/GameplayEffects/GE_FullHealth.GE_FullHealth_C" :`Level` 1.0))

(event `self.ReceiveBeginPlay`
  (set `self.AbilityTagContainer` (struct :`GameplayTags` (struct :`(TagName` "stat.AI"))))
  (`KismetSystemLibrary.Delay` 0.1)
  (`self.SpiderDroneAbilities`))

(fn `GiveMeAbilities`)

(fn `UserConstructionScript`)