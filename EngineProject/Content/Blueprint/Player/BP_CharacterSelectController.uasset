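; Player controller for character selection that sets Game and UI input mode on BeginPlay.
; PlayMediaFile opens a given media source on its MediaPlayer, and StopMediaFile pauses that player rather than closing it.
; Logic to create the WBP_CharacterSelect widget and show the mouse cursor is present but disconnected, so it never runs.
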(event `self.ReceiveBeginPlay`
  (`WidgetBlueprintLibrary.SetInputMode_GameAndUIEx` self null))

(event `self.PlayMediaFile`
  (params (mediaSource :type "FileMediaSource Object Reference"))
  (`MediaPlayer.OpenSource` (`self.MediaPlayer`) mediaSource))

(event `self.StopMediaFile`
  (`MediaPlayer.Pause` (`self.MediaPlayer`)))

(fn `UserConstructionScript`)