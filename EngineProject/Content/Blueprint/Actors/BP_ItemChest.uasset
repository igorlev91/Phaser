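; BP_ItemChest is an item chest actor that plays an opening animation driven by a Timeline.
; At BeginPlay it caches the bottom mesh's world location and rotation.
; The OpenChestAnim event plays OpenTimeline, moving and rolling the lid in relative space while offsetting the base's height and roll from the cached world transform.
; It contains no trigger or item-granting logic; overlap and tick events are disabled.
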(event `self.ReceiveBeginPlay`
  (bind _chestbottommesh (`self.ChestBottomMesh`))
  (set `self.currentLocation` (`SceneComponent.K2_GetComponentLocation` _chestbottommesh))
  (set `self.currentRotaiton` (`SceneComponent.K2_GetComponentRotation` _chestbottommesh)))

(event `self.OpenChestAnim`
  (bind _chestbottommesh (`self.ChestBottomMesh`))
  (bind (_currentlocation_x _currentlocation_y _currentlocation_z) (`KismetMathLibrary.BreakVector` (`self.currentLocation`)))
  (bind (_currentrotaiton_roll _currentrotaiton_pitch _currentrotaiton_yaw) (`KismetMathLibrary.BreakRotator` (`self.currentRotaiton`)))
  (bind (_direction _topmesh_transform _topmesh_rotationx _bottommesh_transformz _bottommesh_rotationx) (`Timeline|OpenTimeline` :!via `PlayFromStart`)
    (:`Update`
      (`SceneComponent.K2_SetRelativeLocation` (`self.ChestTopMesh`) _topmesh_transform false false)
      (`SceneComponent.K2_SetRelativeRotation` (`self.ChestTopMesh`) (`KismetMathLibrary.MakeRotator` _topmesh_rotationx) false false)
      (`SceneComponent.K2_SetWorldLocation` _chestbottommesh (`KismetMathLibrary.MakeVector` _currentlocation_x _currentlocation_y (+ _currentlocation_z _bottommesh_transformz)) false false)
      (`SceneComponent.K2_SetWorldRotation` _chestbottommesh (`KismetMathLibrary.MakeRotator` (+ _currentrotaiton_roll _bottommesh_rotationx) _currentrotaiton_pitch _currentrotaiton_yaw) false false))))

(fn `UserConstructionScript`)