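; BP_FlickeringLight_Stadium is a spotlight actor that flickers on and off between a dim and a normal intensity.
; The construction script sets the normal intensity.
; BeginPlay runs an endless loop: a retriggerable delay of random length between MinTime and MaxTime feeds a FlipFlop that alternates the spotlight between MinFlickerInstensity and Intensity.
; Each pass also sets the light function fade distance to a fixed value.
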(event `self.ReceiveBeginPlay`
  (bind _spotlight (`self.SpotLight`))
  (`KismetSystemLibrary.RetriggerableDelay` (`KismetMathLibrary.RandomFloatInRange` (`self.MinTime`) (`self.MaxTime`)) :!label _label)
  (`/Engine/EditorBlueprintResources/StandardMacros.FlipFlop`
    (:`A`
      (`LightComponent.SetIntensity` _spotlight (`self.MinFlickerInstensity`)))
    (:`B`
      (`LightComponent.SetIntensity` _spotlight (`self.Intensity`))))
  (`LightComponent.SetLightFunctionFadeDistance` (`self.SpotLight`) 200.0)
  (goto _label))

(fn `UserConstructionScript`
  (`LightComponent.SetIntensity` (`self.SpotLight`) (`self.Intensity`)))