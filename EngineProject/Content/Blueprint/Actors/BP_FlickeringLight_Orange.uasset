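; BP_FlickeringLight_Orange is a light actor whose point light flickers at irregular intervals.
; The construction script applies the base Intensity to the PointLight.
; From BeginPlay, a self-looping RetriggerableDelay waits a random time between MinTime and MaxTime, then a FlipFlop alternates the light between the minimum flicker intensity and the base Intensity.
; Each cycle also resets the light function fade distance to a fixed value, with no Tick logic.
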(event `self.ReceiveBeginPlay`
  (bind _pointlight (`self.PointLight`))
  (`KismetSystemLibrary.RetriggerableDelay` (`KismetMathLibrary.RandomFloatInRange` (`self.MinTime`) (`self.MaxTime`)) :!label _label)
  (`/Engine/EditorBlueprintResources/StandardMacros.FlipFlop`
    (:`A`
      (`LightComponent.SetIntensity` _pointlight (`self.MinFlickerInstensity`)))
    (:`B`
      (`LightComponent.SetIntensity` _pointlight (`self.Intensity`))))
  (`LightComponent.SetLightFunctionFadeDistance` (`self.PointLight`) 1.0)
  (goto _label))

(fn `UserConstructionScript`
  (`LightComponent.SetIntensity` (`self.PointLight`) (`self.Intensity`)))